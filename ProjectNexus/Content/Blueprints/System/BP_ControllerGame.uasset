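; BP_ControllerGame is a game controller Blueprint that initializes the player's abilities and mouse input when play begins.
; BeginPlay runs the player setup, then enables click events and shows the mouse cursor.
; Setup caches the ability component by calling GetAbilityComponentMessage on player character 0, then has that component set the starting ability.
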(event EventBeginPlay
  (|CallParentFunction)
  (CallFunction|SetUpPlayer)
  (Variables|Default|SetbEnableClickEvents true)
  (Variables|Default|SetbShowMouseCursor true))

(fn ConstructionScript)

(fn SetUpPlayer
  (CallFunction|SetUpReferences)
  (Default|SetStartingAbility (Variables|Default|GetAbilityComponentRef)))

(fn SetUpReferences
  (bind _abilitycomponent (Class|BPIAbilities|GetAbilityComponent(Message) (Game|GetPlayerCharacter 0)))
  (Variables|Default|SetAbilityComponentRef _abilitycomponent))