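; Game instance that carries player choices and stats across levels: selected character, starting ability, navigation data, kill count and total runs.
; Setter events store these values, and matching getters return them, while the many other interface-style getters are empty stubs returning defaults.
; Setting the first active ability also maps its character-class name to a gameplay tag, added to the AbilitiesTag container of the player character cached on Init.
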(event EventSetSelectedCharacter
  (params (SelectedCharacterClass :type Pawn%20Class%20Reference) (ClassName :type Name :default "None"))
  ;[1 1 1] Receives Message of Selected Character to use in Mission Levels
  (Variables|Default|SetSelectedCharacter SelectedCharacterClass)
  (Variables|Default|SetSelectedCharName ClassName))

(event EventSetNavigationData
  (params (NavPoints :type Integer))
  ;[1 1 1] Receives Message of Selected Character to use in Mission Levels
  (Variables|Default|SetNavigationData NavPoints))

(event EventSetActive1
  (params (Active1 :type Texture%202D%20Object%20Reference) (ActiveName1 :type Name :default "None") (StartTag :type Gameplay%20Tag%20Structure) (ActiveTag :type Gameplay%20Tag%20Structure))
  (Variables|Default|SetStartingAbilityIcon Active1)
  (bind _output_get (Variables|Default|SetStartingAbilityName ActiveName1))
  (switch name _output_get
    (:Mechingineer
      (GameplayTags|AddGameplayTag (Variables|/Game/Blueprints/Characters/BP_BaseCharacterClass.BP_BaseCharacterClass_C|GetAbilitiesTag (Variables|Default|GetCharacterRef)) "(TagName=\"Active.FireBall\")" :!class /Script/GameplayTags.BlueprintGameplayTagLibrary))
    (:WizardLizard
      (GameplayTags|AddGameplayTag (Variables|/Game/Blueprints/Characters/BP_BaseCharacterClass.BP_BaseCharacterClass_C|GetAbilitiesTag (Variables|Default|GetCharacterRef)) "(TagName=\"Active.MagicMissile\")" :!class /Script/GameplayTags.BlueprintGameplayTagLibrary))
    (:Hacker
      (GameplayTags|AddGameplayTag (Variables|/Game/Blueprints/Characters/BP_BaseCharacterClass.BP_BaseCharacterClass_C|GetAbilitiesTag (Variables|Default|GetCharacterRef)) "(TagName=\"Active.ElectricField\")" :!class /Script/GameplayTags.BlueprintGameplayTagLibrary))
    (:Pilot
      (GameplayTags|AddGameplayTag (Variables|/Game/Blueprints/Characters/BP_BaseCharacterClass.BP_BaseCharacterClass_C|GetAbilitiesTag (Variables|Default|GetCharacterRef)) "(TagName=\"Active.Pistol\")" :!class /Script/GameplayTags.BlueprintGameplayTagLibrary))
    (:Warden
      (GameplayTags|AddGameplayTag (Variables|/Game/Blueprints/Characters/BP_BaseCharacterClass.BP_BaseCharacterClass_C|GetAbilitiesTag (Variables|Default|GetCharacterRef)) "(TagName=\"Active.AssaultRifle\")" :!class /Script/GameplayTags.BlueprintGameplayTagLibrary))))

(event EventInit
  (bind _asbp_base_character_class (Utilities|Casting|CastToBP_BaseCharacterClass (Game|Player|GetPlayerPawn 0)))
  (Variables|Default|SetCharacterRef _asbp_base_character_class))

(event EventSetTotalRuns
  (params (Runs :type Integer))
  (Variables|Default|SetTotalRuns Runs))

(event EventSetSaveKillCounter
  (params (KillCount :type Integer))
  (Variables|Default|SetKillCount KillCount))

(fn GetAbility
  (return 0))

(fn GetAbilityComponent
  (return 0))

(fn GetAbilityTag
  (return ""))

(fn GetActive1
  (return (Variables|Default|GetStartingAbilityIcon) (Variables|Default|GetStartingAbilityName) "" ""))

(fn GetActive2
  (return 0 "None"))

(fn GetActive3
  (return 0 "None"))

(fn GetActive4
  (return 0 "None"))

(fn GetAssaultRifleStats
  (return 0 0.0 0.0))

(fn GetIsBreakthrough
  (return false))

(fn GetMaxHPPassiveLvl
  (return 0))

(fn GetMissionType
  (return ""))

(fn GetNavigationData
  (return (Variables|Default|GetNavigationData)))

(fn GetOrbitSpawner
  (return 0))

(fn GetPassive1
  (return 0 "None" 0))

(fn GetPassive2
  (return 0 "None" 0))

(fn GetPassive3
  (return 0 "None" 0))

(fn GetPlayerCurrentHealth
  (return 0.0))

(fn GetPlayerDeathStatus
  (return false))

(fn GetPlayerLevel
  (return 0))

(fn GetPlayerMaxHealth
  (return 0.0))

(fn GetPlayerXP
  (return 0.0))

(fn GetProjectileSpawner
  (return 0))

(fn GetRunKillCounter
  (return 0))

(fn GetSaveKillCounter
  (return (Variables|Default|GetKillCount)))

(fn GetSelectedCharacter
  (return (Variables|Default|GetSelectedCharacter) (Variables|Default|GetSelectedCharName)))

(fn GetTotalRuns
  (return (Variables|Default|GetTotalRuns)))

(fn GetXptoLevel
  (return 0.0))

(fn Heal
  (params (HealAmount :type Float%20%28double-precision%29))
  (return 0.0))

(fn TakeDamage
  (params (DamgeInfo :type BPS%20Damage%20Info%20Structure))
  (return false))