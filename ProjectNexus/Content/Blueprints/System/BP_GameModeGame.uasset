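; BP_GameModeGame is the gameplay game mode that spawns the player's selected character and shows the combat UI.
; On BeginPlay it creates WBP_CombatUI for the first player controller, adds it to the viewport and sets Game and UI input mode.
; Its GetDefaultPawnClassForController override reads the selected character class from the Game Instance, falling back to the parent's default pawn class when that class is invalid.
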(event EventBeginPlay
  (bind _returnvalue (Game|GetPlayerController 0))
  (bind _returnvalue_2 (UserInterface|CreateWidget "/Game/UI/WBP_CombatUI.WBP_CombatUI_C" _returnvalue))
  (UserInterface|Viewport|AddtoViewport _returnvalue_2 0)
  (Input|SetInputModeGameandUI _returnvalue 0 "DoNotLock" true false))

(fn ConstructionScript)

(fn GetDefaultPawnClassforController
  (params (InController :type Controller%20Object%20Reference))
  (bind _returnvalue (|CallParentFunction InController))
  (bind _selectedcharacterclass (Class|BPIMissionSetup|GetSelectedCharacter(Message) (Game|GetGameInstance)))
  (if (Utilities|IsValidClass _selectedcharacterclass)
    (return _selectedcharacterclass)
    (else
      (return _returnvalue))))