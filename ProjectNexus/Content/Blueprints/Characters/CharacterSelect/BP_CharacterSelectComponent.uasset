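; Actor component for character selection that makes its owning actor a hoverable, clickable class choice.
; On BeginPlay it binds the owner's cursor and click events, using custom depth on the owner's skeletal mesh as a hover highlight.
; Clicks toggle a selected flag; when set, it sends the class Blueprint from DT_Classes to the GameInstance, opens TestLevel and sets Game and UI input.
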(event Custom|OnMouseClick
  (params (TouchedActor :type Actor%20Object%20Reference) (ButtonPressed :type Key%20Structure :default "None"))
  (bind _output_get (Variables|Default|SetIsClicked? (not (Variables|Default|GetIsClicked?))))
  (Utilities|IsValid (Variables|Default|GetSkeletalRef)
    (:Is%20Valid
      (if _output_get
        (Class|BPIMissionSetup|SetSelectedCharacter(Message) (Game|GetGameInstance) (.ClassBP (CallFunction|GetCharacterData)) "None")
        (Game|OpenLevel(byName) "TestLevel")
        (Input|SetInputModeGameandUI (Game|GetPlayerController 0) 0 "DoNotLock" true false)))))

(event Custom|OnMouseHover
  (params (TouchedActor :type Actor%20Object%20Reference))
  (Rendering|SetRenderCustomDepth (Variables|Default|GetSkeletalRef) true))

(event Custom|OnMouseExit
  (params (TouchedActor :type Actor%20Object%20Reference))
  (Rendering|SetRenderCustomDepth (Variables|Default|GetSkeletalRef) false))

(event EventBeginPlay
  (bind _returnvalue (Components|GetOwner))
  (bind _returnvalue_2 (Actor|GetComponentbyClass _returnvalue "/Script/Engine.SkeletalMeshComponent"))
  (EventDispatchers|BindEventtoOnClicked _returnvalue (delegate Custom|OnMouseClick))
  (Utilities|IsValid _returnvalue_2
    (:Is%20Valid
      (Variables|Default|SetSkeletalRef _returnvalue_2)
      (EventDispatchers|BindEventtoOnBeginCursorOver _returnvalue (delegate Custom|OnMouseHover))
      (EventDispatchers|BindEventtoOnEndCursorOver _returnvalue (delegate Custom|OnMouseExit)))))

(fn GetCharacterData
  (bind _returnvalue (Utilities|GetDataTableRow "/Game/Blueprints/DataTables/DT_Classes.DT_Classes" (.RowName (Utilities|Struct|BreakDataTableRowHandle (Variables|Default|GetCharacterData))))
    (:then
      (return (.ClassName (Utilities|Struct|BreakBPS_Classes _returnvalue)) (.Description (Utilities|Struct|BreakBPS_Classes _returnvalue)) (.ClassIcon (Utilities|Struct|BreakBPS_Classes _returnvalue)) (.ClassBP (Utilities|Struct|BreakBPS_Classes _returnvalue)) (.IconColor (Utilities|Struct|BreakBPS_Classes _returnvalue))))))