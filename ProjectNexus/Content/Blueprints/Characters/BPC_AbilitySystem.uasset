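; Ability component that runs auto-firing weapons and spells, starting with one chosen by the selected character's class.
; Leveling functions adjust stats and restart looping timers by function name, which spawn projectiles or AOEs; guns track clips and reloads.
; Milestone levels store paired breakthrough options, and BreakthroughTrigger switches on gameplay tags to apply the upgrade.
; Several abilities are WIP or await the new damage system, and many breakthroughs only print.
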(event Custom|GravityWell
  (bind _playerref (Variables|Default|GetPlayerRef))
  (bind _returnvalue (Transformation|GetActorLocation _playerref))
  ;[0.3451 0.8 1] Gravity Well | Needs to be revamped to the new damage system
  (Utilities|Time|SetTimerbyFunctionName 0 "GravityWell" (Variables|GravityWell|GetGravityWellFireRate) true true)
  (bind (_outhit _returnvalue_2) (Collision|LineTraceByChannel _returnvalue (* _returnvalue "1.000000,1.000000,-1000.000000") "TraceTypeQuery1" false (Utilities|Array|MakeArray 0) "None"))
  (if _returnvalue_2
    (bind _returnvalue_3 (Game|SpawnActorfromClass "/Game/Blueprints/Melee/BP_GravityWell.BP_GravityWell_C" (Math|Transform|MakeTransform (.Location (Collision|BreakHitResult _outhit)) "0, 0, 0" "1.000000,1.000000,1.000000") "Undefined" "MultiplyWithRoot" 0 5.0 5.0 2e+02 true true false 0))
    (EventDispatchers|AssignOnAOEOverlapActor _returnvalue_3 (delegate Custom|DamageEnemyOverTime))))

(event Custom|AssaultRifle
  (bind _assaultrifledamagerange (Variables|AssaultRifle|GetAssaultRifleDamageRange))
  ;[0 0 1] AssaultRifle | WIP
  (if (Variables|AssaultRifle|GetARClipFull?)
    (bind _projectilespawn (Class|BPIPlayerStats|GetProjectileSpawner(Message) (Components|GetOwner)))
    (bind _returnvalue (Actor|GetActorOfClass "/Game/Blueprints/Enemies/BP_ParentEnemyClass.BP_ParentEnemyClass_C"))
    (Game|SpawnActorfromClass "/Game/Blueprints/Projectiles/BP_AssaultRifle.BP_AssaultRifle_C" (Transformation|GetWorldTransform _projectilespawn) "Undefined" "MultiplyWithRoot" 0 1.5e+03 0.0 _returnvalue false false (Math|Random|RandomFloatinRange (.MinValue (Math|Float|MinOfFloatArray _assaultrifledamagerange)) (.MaxValue (Math|Float|MaxOfFloatArray _assaultrifledamagerange))) 0)
    (bind _result (Math|Integer|DecrementInt (Variables|AssaultRifle|GetARClipCurrent))
      (:%20%20
        (Development|PrintString (Utilities|String|ToString(Integer) _result))
        (if (== _result 0)
          (bind _output_get (Variables|AssaultRifle|SetARClipFull? false))
          (Development|PrintString (Utilities|String|ToString(Boolean) _output_get)))))
    (else
      (|ARReload))))

(event Custom|Pistol
  ;[0 0 1] Pistol | WIP
  (if (Variables|Pistol|GetPistolClipFull?)
    (bind _projectilespawn (Class|BPIPlayerStats|GetProjectileSpawner(Message) (Components|GetOwner)))
    (bind _returnvalue (Actor|GetActorOfClass "/Game/Blueprints/Enemies/BP_ParentEnemyClass.BP_ParentEnemyClass_C"))
    (Game|SpawnActorfromClass "/Game/Blueprints/Projectiles/BP_AssaultRifle.BP_AssaultRifle_C" (Math|Transform|MakeTransform (Transformation|GetWorldLocation _projectilespawn) "0, 0, 0" "0.300000,0.300000,0.300000") "Undefined" "MultiplyWithRoot" 0 2e+03 0.0 _returnvalue false true (Math|Random|RandomFloatinRange (.MinValue (Math|Float|MinOfFloatArray (Variables|Pistol|GetPistolDamage))) (.MaxValue (Math|Float|MaxOfFloatArray (Variables|Pistol|GetPistolDamage)))) 0)
    (bind _result (Math|Integer|DecrementInt (Variables|Pistol|GetPistolClipCurrent))
      (:%20%20
        (Development|PrintString (Utilities|String|ToString(Integer) _result))
        (if (== _result 0)
          (bind _output_get (Variables|Pistol|SetPistolClipFull? false))
          (Development|PrintString (Utilities|String|ToString(Boolean) _output_get)))))
    (else
      (|PistolReload))))

(event Custom|TriggerBreakthrough
  ;[0 0 1] Controls the Breakthrough Triggers and abilities
  (CallFunction|BreakthroughTrigger))

(event Custom|FireBall
  (bind _fireballdamagerange (Variables|FireBall|GetFireBallDamageRange))
  ;[0 0 1] Fire Ball
  (bind _projectilespawn (Class|BPIPlayerStats|GetProjectileSpawner(Message) (Components|GetOwner)))
  (bind _returnvalue (Actor|GetActorOfClass "/Game/Blueprints/Enemies/BP_ParentEnemyClass.BP_ParentEnemyClass_C"))
  (Game|SpawnActorfromClass "/Game/Blueprints/Projectiles/BP_FireBall.BP_FireBall_C" (Math|Transform|MakeTransform (Transformation|GetWorldLocation _projectilespawn) "0, 0, 0" (Variables|FireBall|GetFireBallSize)) "Undefined" "MultiplyWithRoot" 0 (Variables|FireBall|GetFireBallSpeed) 0.0 _returnvalue false true (Math|Random|RandomFloatinRange (.MinValue (Math|Float|MinOfFloatArray _fireballdamagerange)) (.MaxValue (Math|Float|MaxOfFloatArray _fireballdamagerange))) 0))

(event Custom|LightningBolt
  ;[0.3451 0.8 1] Lightning Bolt | Needs to be revamped to the new damage system
  (Utilities|Time|SetTimerbyFunctionName 0 "LightningBolt" (Variables|LightningBolt|GetLightningBoltFireRate) true)
  (bind _returnvalue (Actor|GetActorOfClass "/Game/Blueprints/Enemies/BP_ParentEnemyClass.BP_ParentEnemyClass_C"))
  (bind _returnvalue_2 (Game|SpawnActorfromClass "/Game/Blueprints/Melee/AOE_LightningBolt.AOE_LightningBolt_C" (Math|Transform|MakeTransform (Transformation|GetActorLocation (Variables|Default|GetPlayerRef)) "0, 0, 0" "1.000000,1.000000,1.000000") "Undefined" "MultiplyWithRoot" 0 1.0 _returnvalue 2.5e+02 true true true (Variables|Default|GetPlayerRef)))
  (EventDispatchers|AssignOnAOEOverlapActor _returnvalue_2 (delegate Custom|DamageEnemyAoe)))

(event Custom|DamageEnemyOverTime
  (params (Actor :type Actor%20Object%20Reference))
  ;[0.3451 0.8 1] Gravity Well | Needs to be revamped to the new damage system
  (Class|BPIPlayerStats|TakeDamage(Message) Actor (Utilities|Struct|MakeBPS_DamageInfo (Variables|GravityWell|GetGravityWellDamage) "NewEnumerator3")))

(event Custom|Damage%20Enemy
  (params (Component :type Actor%20Component%20Object%20Reference) (bReset :type Boolean))
  ;[0.3451 0.8 1] Double Bladed Lance | Needs to be revamped to new damage system
  (Class|BPIPlayerStats|TakeDamage(Message) Component (Utilities|Struct|MakeBPS_DamageInfo 5e+01 "NewEnumerator1" "NewEnumerator2" false true)))

(event Custom|MagicMissile
  ;[0 0.01 1] Magic Missile v2
  (for _index (range 0 (- (Variables|MagicMissile|GetMagicMissileCount) 1))
    (bind _projectilespawn (Class|BPIPlayerStats|GetProjectileSpawner(Message) (Components|GetOwner)))
    (bind _returnvalue (Actor|GetActorOfClass "/Game/Blueprints/Enemies/BP_ParentEnemyClass.BP_ParentEnemyClass_C"))
    (Game|SpawnActorfromClass "/Game/Blueprints/Projectiles/BP_ProjectileMagicMissile.BP_ProjectileMagicMissile_C" (Math|Transform|MakeTransform (+ (Transformation|GetSocketLocation _projectilespawn "AOESocket") (* (Math|Vector|GetForwardVector (Math|Rotator|CombineRotators (Transformation|GetActorRotation (Components|GetOwner)) (Math|Rotator|MakeRotator 0.0 0.0 (Math|Conversions|ToFloat(Integer) (* _index (/ 360 (Variables|MagicMissile|GetMagicMissileCount))))))) 100)) (Math|Rotator|CombineRotators (Transformation|GetActorRotation (Components|GetOwner)) (Math|Rotator|MakeRotator 0.0 0.0 (Math|Conversions|ToFloat(Integer) (* _index (/ 360 (Variables|MagicMissile|GetMagicMissileCount)))))) "1.000000,1.000000,1.000000") "Undefined" "MultiplyWithRoot" 0 (Variables|MagicMissile|GetMagicMissileSpeed) 0.0 _returnvalue (Variables|MagicMissile|GetMagicMissileHoming) false 1e+02 0)))

(event Custom|DamageEnemyAoe
  (params (Actor :type Actor%20Object%20Reference))
  ;[0.3451 0.8 1] Lightning Bolt | Needs to be revamped to the new damage system
  (Class|BPIPlayerStats|TakeDamage(Message) Actor (Utilities|Struct|MakeBPS_DamageInfo (Variables|LightningBolt|GetLightningBoltDamage) "NewEnumerator3")))

(event Custom|ElectricField
  ;[0 0 1] Electric Field | WIP
  (bind _projectilespawn (Class|BPIPlayerStats|GetProjectileSpawner(Message) (Components|GetOwner)))
  (bind _returnvalue (Game|SpawnActorfromClass "/Game/Blueprints/Melee/BP_AoE_Explosion.BP_AoE_Explosion_C" (Math|Transform|MakeTransform (Transformation|GetWorldLocation _projectilespawn) "0, 0, 0" "1.000000,1.000000,1.000000") "Undefined" "MultiplyWithRoot" 0 2e+02 true true true 0))
  (Transformation|AttachComponentToComponent _returnvalue _projectilespawn "AOESocket" "SnapToTarget" "SnapToTarget" "SnapToTarget" true))

(event Custom|DoubleBladedLance
  ;[0.3451 0.8 1] Double Bladed Lance | Needs to be revamped to new damage system
  (Utilities|Time|SetTimerbyFunctionName 0 "DoubleBladeLance" 2.0 true)
  (bind _returnvalue (Niagara|SpawnSystematLocation "/Game/Hack_And_Slash_FX/VFX_Niagara/Slashes/NS_Sakura_Slash.NS_Sakura_Slash" (Transformation|GetWorldLocation (Variables|/Game/Blueprints/Characters/BP_BaseCharacterClass.BP_BaseCharacterClass_C|GetProjectileSpawnLocation (Variables|Default|GetPlayerRef)))))
  (Components|Activation|BindEventtoOnComponentActivated _returnvalue (delegate Custom|Damage%20Enemy))
  (Collision|IgnoreActorwhenMoving (Variables|/Script/Engine.Character|GetCapsuleComponent (Variables|Default|GetPlayerRef)) 0 true))

(event EventBeginPlay
  ;[1 1 1] Character Reference
  (bind _outactors (Actor|GetAllActorsOfClass "/Game/Blueprints/Characters/BP_BaseCharacterClass.BP_BaseCharacterClass_C"))
  (Variables|Default|SetPlayerRef (Utilities|Array|Get(acopy) _outactors)))

(event EventSetWeaponStatusTag
  (params (StatusTag :type Gameplay%20Tag%20Container%20Structure))
  (Variables|Default|SetStatusTags StatusTag))

(fn GetAbilityData
  (bind _returnvalue (Utilities|GetDataTableRow "/Game/Blueprints/DataTables/DT_Abilities.DT_Abilities" (.RowName (Utilities|Struct|BreakDataTableRowHandle (Variables|Default|GetAbilityData))))
    (:then
      (return (.Name (Utilities|Struct|BreakBPS_Abilities _returnvalue)) (.Type (Utilities|Struct|BreakBPS_Abilities _returnvalue)) (.Description (Utilities|Struct|BreakBPS_Abilities _returnvalue)) (.Icon (Utilities|Struct|BreakBPS_Abilities _returnvalue)) (.Class (Utilities|Struct|BreakBPS_Abilities _returnvalue)) (.AbilitySelected (Utilities|Struct|BreakBPS_Abilities _returnvalue))))
    (:RowNotFound
      (return "None" "None" "" 0 "" ""))))

(fn MagicMissileLeveling
  (bind _result (Math|Integer|IncrementInt (Variables|MagicMissile|GetMagicMissileLevel))
    (:%20%20
      (Development|PrintString (Utilities|String|ToString(Integer) _result))
      (switch int (Variables|MagicMissile|GetMagicMissileLevel)
        (:1
          _)
        (:2
          (|MMLv2))
        (:3
          (|MMLv3
            (:%20%20
              _)))
        (:4
          (|MMLv4))
        (:5
          (|MMLv5))
        (:6
          (|MMLv6))
        (:7
          (|MMLv7))
        (:8
          (|MMLv8))
        (:9
          (|MMLv9))
        (:10
          (|MMLv10)))
      (Abilities|Active|MagicMissile|MagicMissileSetUp))))

(fn SetStartingAbility
  (bind _returnvalue (Game|GetGameInstance))
  (Class|BPIAbilities|GetActive1(Message) _returnvalue)
  (bind _classname (Class|BPIMissionSetup|GetSelectedCharacter(Message) _returnvalue))
  (switch name _classname
    (:Mechingineer
      (Abilities|Active|FireBall|FireBallLeveling))
    (:Wizard%20Lizard
      (Abilities|Active|MagicMissile|MagicMissileLeveling))
    (:Hacker
      (Abilities|Active|ElectricField|ElectricFieldLeveling))
    (:Pilot
      (Abilities|Active|Pistol|PistolLeveling))
    (:Warden
      (Abilities|Active|AssaultRifle|AssaultRifleLeveling))))

(fn MagicMissileSetUp
  (Utilities|Time|SetTimerbyFunctionName 0 "MagicMissile" (Utilities|CalculateTimer (Variables|MagicMissile|GetMagicMissileFireRate)) true)
  (CallFunction|MagicMissile))

(fn AssaultRifleLeveling
  (bind _result (Math|Integer|IncrementInt (Variables|AssaultRifle|GetAssaultRifleLevel))
    (:%20%20
      (Development|PrintString (Utilities|String|ToString(Integer) _result))
      (switch int _result
        (:1
          _)
        (:2
          (|ARLv2))
        (:3
          (|ARLv3))
        (:4
          (|ARLv4))
        (:5
          (|ARLv5))
        (:6
          (|ARLv6))
        (:7
          (|ARLv7))
        (:8
          (|ARLv8))
        (:9
          (|ARLv9)))
      (Abilities|Active|AssaultRifle|AssaultRifleSetUp))))

(fn AssaultRifleSetUp
  (Utilities|Time|SetTimerbyFunctionName 0 "AssaultRifle" (Variables|AssaultRifle|GetAssaultRifleFireRate) true)
  (CallFunction|AssaultRifle))

(fn ElectricFieldSetUp
  (Utilities|Time|SetTimerbyFunctionName 0 "ElectricField" (Utilities|CalculateTimer (Variables|ElectricField|GetElectricFieldFireRate)) true)
  (CallFunction|ElectricField))

(fn ElectricFieldLeveling
  (switch int (Variables|ElectricField|GetElectricFieldLevel)
    (:1
      (Abilities|Active|ElectricField|ElectricFieldSetUp))))

(fn FireBallSetUp
  (Utilities|Time|SetTimerbyFunctionName 0 "FireBall" (Utilities|CalculateTimer (Variables|FireBall|GetFireBallFireRate)) true)
  (CallFunction|FireBall))

(fn FireBallLeveling
  (bind _result (Math|Integer|IncrementInt (Variables|FireBall|GetFireBallLevel))
    (:%20%20
      (Development|PrintString (Utilities|String|ToString(Integer) _result))
      (switch int (Variables|FireBall|GetFireBallLevel)
        (:1
          (Abilities|Active|FireBall|FireBallSetUp))
        (:2
          (|FireBallLvl2)
          (Abilities|Active|FireBall|FireBallSetUp :!label _label))
        (:3
          (|FireBallLvl3)
          (goto _label))
        (:4
          (|FireBallLvl4)
          (goto _label))
        (:5
          (|FireBallLvl5)
          (goto _label))
        (:6
          (|FireBallLvl6)
          (goto _label))
        (:7
          (|FireBallLvl7)
          (goto _label))
        (:8
          (|FireBallLvl8)
          (goto _label))
        (:9
          (|FireBallLvl9)
          (goto _label))
        (:10
          (|FireBallLvl10)
          (goto _label))))))

(fn PistolSetUp
  (Utilities|Time|SetTimerbyFunctionName 0 "Pistol" (Variables|Pistol|GetPistolFireRate) true))

(fn PistolLeveling
  (bind _result (Math|Integer|IncrementInt (Variables|Pistol|GetPistolLevel))
    (:%20%20
      (Development|PrintString (Utilities|String|ToString(Integer) _result))
      (switch int _result
        (:1
          _)
        (:2
          (|PistolLv2))
        (:3
          (|PistolLv3))
        (:4
          (|PistolLvl4))
        (:5
          (|PistolLv5))
        (:6
          (|PistolLv6))
        (:7
          (|PistolLvl7))
        (:8
          (|PistolLv8))
        (:9
          (|PistolLv9))
        (:10
          (|PistolLvl10)))
      (Abilities|Active|Pistol|PistolSetUp))))

(fn Breakthrough
  (Game|SetGamePaused true)
  (bind _returnvalue (UserInterface|CreateWidget "/Game/UI/WBP_Breakthroughs.WBP_Breakthroughs_C"))
  (UserInterface|Viewport|AddtoViewport _returnvalue 0))

(fn GetBreakthrough
  (params (Breakthrough? :type Boolean) (Breakthrough1 :type Gameplay%20Tag%20Container%20Structure) (Breakthrough2 :type Gameplay%20Tag%20Container%20Structure) (BreakthroughImage1 :type Texture%202D%20Object%20Reference) (BreakthroughImage2 :type Texture%202D%20Object%20Reference))
  (Variables|Breakthroughs|SetBreakthrough? Breakthrough?)
  (Variables|Breakthroughs|SetBreakthrough1 Breakthrough1)
  (Variables|Breakthroughs|SetBreakthrough2 Breakthrough2)
  (Variables|Breakthroughs|SetBreakthroughImage1 BreakthroughImage1)
  (Variables|Breakthroughs|SetBreakthroughImage2 BreakthroughImage2))

(fn BreakthroughTrigger
  (|SwitchGameplayTagContainer (Variables|Breakthroughs|GetBreakthroughTagContainer)
    (:%28GameplayTags=%28%28TagName="Active.FireBall.KnockBack"%29%29%29
      (|FireBallBreakThroughTriggers :!label _label))
    (:%28GameplayTags=%28%28TagName="Active.FireBall.FireBoulder"%29%29%29
      (goto _label execute2))
    (:%28GameplayTags=%28%28TagName="Active.FireBall.LavaPit"%29%29%29
      (goto _label execute3))
    (:%28GameplayTags=%28%28TagName="Active.FireBall.ClusterBomb"%29%29%29
      (goto _label execute4))
    (:%28GameplayTags=%28%28TagName="Active.FireBall.FiringSquad"%29%29%29
      (goto _label execute5))
    (:%28GameplayTags=%28%28TagName="Active.FireBall.Implosion"%29%29%29
      (goto _label execute6))
    (:%28GameplayTags=%28%28TagName="Active.Pistol.PiercingAmmo"%29%29%29
      (|PistolBreakthroughTriggers :!label _label_2))
    (:%28GameplayTags=%28%28TagName="Active.Pistol.HollowPointAmmo"%29%29%29
      (goto _label_2 execute2))
    (:%28GameplayTags=%28%28TagName="Active.Pistol.RapidFire"%29%29%29
      (goto _label_2 execute3))
    (:%28GameplayTags=%28%28TagName="Active.Pistol.ChargeShot"%29%29%29
      (goto _label_2 execute4))
    (:%28GameplayTags=%28%28TagName="Active.Pistol.Freezerounds"%29%29%29
      (goto _label_2 execute5))
    (:%28GameplayTags=%28%28TagName="Active.Pistol.PlasmaAmmo"%29%29%29
      (goto _label_2 execute6))
    (:%28GameplayTags=%28%28TagName="Active.MagicMissile.Split"%29%29%29
      (|MagicMissileBreakthroughTriggers :!label _label_3))
    (:%28GameplayTags=%28%28TagName="Active.MagicMissile.Velocity"%29%29%29
      (goto _label_3 execute2))
    (:%28GameplayTags=%28%28TagName="Active.MagicMissile.Attunement"%29%29%29
      (goto _label_3 execute3))
    (:%28GameplayTags=%28%28TagName="Active.MagicMissile.Fracture"%29%29%29
      (goto _label_3 execute4))
    (:%28GameplayTags=%28%28TagName="Active.MagicMissile.ArcaneTorrent"%29%29%29
      (goto _label_3 execute5))
    (:%28GameplayTags=%28%28TagName="Active.MagicMissile.DeathBlossom"%29%29%29
      (goto _label_3 execute6))))

(fn MultiplyArrayValues
  (params (Array%20Input :type Array%20of%20Floats%20%28double-precision%29) (Multiplier :type Float%20%28double-precision%29))
  (for (_array_element _array_index) Array%20Input
    (Utilities|Array|SetArrayElem Array%20Input _array_index (* _array_element Multiplier)))
  (return))

(fn ClipController
  (params (BulletCount :type Integer))
  (bind _result (Math|Integer|DecrementInt BulletCount)
    (:%20%20
      (if (== _result 0)
        (Variables|Pistol|SetPistolClipFull? false)
        (return)))))

(fn GetAbility
  (return 0))

(fn GetAbilityComponent
  (return 0))

(fn GetActive1
  (return 0 "None" "" ""))

(fn GetActive2
  (return 0 "None"))

(fn GetActive3
  (return 0 "None"))

(fn GetActive4
  (return 0 "None"))

(fn GetAssaultRifleStats
  (return (Variables|AssaultRifle|GetAssaultRifleLevel) 0.0 0.0))

(fn GetIsBreakthrough
  (return (Variables|Breakthroughs|GetBreakthrough?)))

(fn GetMaxHPPassiveLvl
  (return 0))

(fn GetMissionType
  (return ""))

(fn GetNavigationData
  (return 0))

(fn GetPassive1
  (return 0 "None" 0))

(fn GetPassive2
  (return 0 "None" 0))

(fn GetPassive3
  (return 0 "None" 0))

(fn GetRunKillCounter
  (return 0))

(fn GetSaveKillCounter
  (return 0))

(fn GetSelectedCharacter
  (return 0 "None"))

(fn GetWeaponStatusTag
  (return (Variables|Default|GetStatusTags)))