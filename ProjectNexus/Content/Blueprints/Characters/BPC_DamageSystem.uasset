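; Actor component for a damage system that tracks health, death, invincibility and interruptibility for its owner.
; Heal adds to current health, clamped to the maximum, while the owner is alive.
; TakeDamage's entry is unwired, so its logic never runs: a CanBeDamaged macro gate, health subtraction, then OnDeath or OnDamageResponse dispatcher calls.
; That logic takes a DamageInfo struct whose flags can override invincibility and force interrupts.
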(event EventBeginPlay)

(event EventTick
  (params (DeltaSeconds :type Float%20%28single-precision%29)))

(fn Heal
  (params (HealAmount :type Float%20%28double-precision%29))
  (if (not (Variables|Default|GetIsDead?))
    (bind _output_get (Variables|Default|SetCurrentHealth (Math|Float|Clamp(Float) (+ HealAmount (Variables|Default|GetCurrentHealth)) 0.0 (Variables|Default|GetMaxHealth))))
    (return _output_get)))

(fn TakeDamage
  (params (DamageInfo :type BPS%20Damage%20Info%20Structure)))