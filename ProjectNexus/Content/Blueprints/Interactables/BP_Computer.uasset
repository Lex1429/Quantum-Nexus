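; BP_Computer is an interactable computer that adds a random amount to the Game Instance's NavigationDataMessage value once its progress bar empties.
; Interact starts DrainProgressBar, which lowers the bar in small steps by calling itself after a short Delay while ShouldDrain is true.
; At zero it clears ShouldDrain, grants the random amount and swaps the Computer's material.
; The Sphere overlap events are empty.
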(event OnComponentBeginOverlap(Sphere)
  (params (OverlappedComponent :type Primitive%20Component%20Object%20Reference) (OtherActor :type Actor%20Object%20Reference) (OtherComp :type Primitive%20Component%20Object%20Reference) (OtherBodyIndex :type Integer) (bFromSweep :type Boolean) (SweepResult :type Hit%20Result%20Structure%20%28by%20ref%29)))

(event OnComponentEndOverlap(Sphere)
  (params (OverlappedComponent :type Primitive%20Component%20Object%20Reference) (OtherActor :type Actor%20Object%20Reference) (OtherComp :type Primitive%20Component%20Object%20Reference) (OtherBodyIndex :type Integer)))

(event Custom|DrainProgressBar
  (bind _returnvalue (Game|GetGameInstance))
  (if (Variables|Default|GetShouldDrain?)
    (bind _output_get (Variables|Default|SetProgressBarAmount (Math|Float|Clamp(Float) (- (Variables|Default|GetProgressBarAmount) 0.5) 0.0 (Variables|Default|GetProgressBarMax))))
    (if (== _output_get 0.0)
      (Variables|Default|SetShouldDrain? false)
      (bind _navdatapoints (Class|BPIMissionSetup|GetNavigationData(Message) _returnvalue))
      (Class|BPIMissionSetup|SetNavigationData(Message) _returnvalue (+ _navdatapoints (Math|Random|RandomIntegerinRange 3 10)))
      (Rendering|Material|SetMaterial (Variables|Default|GetComputer) 0 "/Game/PolygonSciFiSpace/Materials/Alternates/MAT_PolygonSciFiSpace_04_A.MAT_PolygonSciFiSpace_04_A")
      (else
        (Utilities|FlowControl|Delay 0.01)
        (CallFunction|DrainProgressBar)))))

(event EventBeginPlay
  (|CallParentFunction) ; This node is disabled and will not be called.\nDrag off pins to build functionality.
)

(event Collision|EventActorBeginOverlap
  (params (OtherActor :type Actor%20Object%20Reference))
  (|CallParentFunction OtherActor) ; This node is disabled and will not be called.\nDrag off pins to build functionality.
)

(event EventTick
  (params (DeltaSeconds :type Float%20%28single-precision%29))
  (|CallParentFunction DeltaSeconds) ; This node is disabled and will not be called.\nDrag off pins to build functionality.
)

(event EventInteract
  (CallFunction|DrainProgressBar))

(fn ConstructionScript
  (|CallParentFunction))