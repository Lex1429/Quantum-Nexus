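; BP_DamageNumberActor is a world actor that shows a damage number as a floating, physically tossed popup.
; On BeginPlay it passes its Damage value to the WBP_DamageInfo widget in its Widget component and launches its StaticMesh with a random upward, sideways velocity impulse.
; The actor destroys itself when the widget signals that its lifetime is over.
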(event Custom|DestroyWidget
  (Actor|DestroyActor))

(event EventBeginPlay
  (bind _aswbp_damage_info (Utilities|Casting|CastToWBP_DamageInfo (UserInterface|GetUserWidgetObject (Variables|Default|GetWidget))))
  (EventDispatchers|BindEventtoWidgetLifetimeOver _aswbp_damage_info (delegate Custom|DestroyWidget))
  (Default|SetDamageValue _aswbp_damage_info (Variables|Default|GetDamage))
  (Physics|AddImpulse (Variables|Default|GetStaticMesh) (Math|Vector|MakeVector (Math|Random|RandomFloatinRange -4e+02 4e+02) (Math|Random|RandomFloatinRange -4e+02 4e+02) (Math|Random|RandomFloatinRange 4e+02 8e+02)) "None" true))

(fn ConstructionScript)