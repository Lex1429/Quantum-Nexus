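; BP_ReloadingText is a short-lived actor that shows a WBP_Reloading widget as floating reload text.
; On BeginPlay it launches its static mesh with a random upward and sideways velocity-change impulse, so it pops into the air.
; It binds to the widget's lifetime-over event and destroys itself when that fires.
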(event Custom|CustomEvent
  (Actor|DestroyActor))

(event EventBeginPlay
  (bind _aswbp_reloading (Utilities|Casting|CastToWBP_Reloading (UserInterface|GetUserWidgetObject (Variables|Default|GetWidget))))
  (EventDispatchers|BindEventtoWidgetLifetimeOver _aswbp_reloading (delegate Custom|CustomEvent))
  (Physics|AddImpulse (Variables|Default|GetStaticMesh) (Math|Vector|MakeVector (Math|Random|RandomFloatinRange -4e+02 4e+02) (Math|Random|RandomFloatinRange -4e+02 4e+02) (Math|Random|RandomFloatinRange 4e+02 8e+02)) "None" true))

(fn ConstructionScript)