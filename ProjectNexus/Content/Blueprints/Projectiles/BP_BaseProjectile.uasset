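; Base projectile Blueprint with configurable speed, gravity, optional homing and auto-aim at a target, expiring after five seconds.
; Construction configures ProjectileMovement; BeginPlay plays the firing sound and, with auto-aim, redirects velocity and ignores the shooter.
; Sphere collisions fire an impact dispatcher, spawn effects and sound, and destroy it unless bouncing.
; A separate Hit event applies damage, and helper functions provide looping burn damage and stored hit data.
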(event OnComponentHit(Sphere1)
  (params (HitComponent :type Primitive%20Component%20Object%20Reference) (OtherActor :type Actor%20Object%20Reference) (OtherComp :type Primitive%20Component%20Object%20Reference) (NormalImpulse :type Vector :default "0, 0, 0") (Hit :type Hit%20Result%20Structure%20%28by%20ref%29))
  (bind _location (Collision|BreakHitResult Hit))
  ;[1 0.1407 0.9913] Particle system and sound generation system
  (Collision|IgnoreActorwhenMoving (Variables|Default|GetMesh) (Game|GetPlayerController 0) false)
  (Default|CallOnProjectileImpact OtherActor Hit)
  (Niagara|SpawnSystematLocation (Variables|Effects|GetEmitter%20Template) _location)
  (Audio|PlaySoundatLocation (Variables|Sounds|GetImpactSound) _location "0, 0, 0" 1.0 1.0 0.0 0 0 0 0)
  (if (not (Variables|Default|GetBounce?))
    (Actor|DestroyActor)))

(event Custom|RotateToTarget
  ;[0 1 0] Auto Aim System
  (Variables|Target|GetTarget
    (:then
      (Variables|/Script/Engine.MovementComponent|SetVelocity (Variables|Default|GetProjectileMovement) (* (Math|Vector|GetUnitDirection(Vector) (Transformation|GetActorLocation) (Transformation|GetActorLocation (Variables|Target|GetTarget))) (Variables|ProjectileSettings|GetSpeed))))
    (:else)))

(event EventBeginPlay
  (bind _returnvalue (Game|GetInstigator))
  ;[0 1 0] If AutoAim is on, will aim to target after spawning. Also stops projectile from coliding with player.
  (Utilities|FlowControl|Sequence
    (:then_0
      (if (Variables|ProjectileSettings|GetAutoAim?)
        (CallFunction|RotatetoTarget)
        (Collision|IgnoreActorwhenMoving (Variables|Default|GetSphere1) (select (Utilities|IsValid _returnvalue) _returnvalue (Components|GetOwner)) true)))
    (:then_1
      (Utilities|FlowControl|Delay 5.0)
      (Actor|DestroyActor))
    (:then_2
      (Audio|PlaySoundatLocation (Variables|Default|GetFireingSound) (Transformation|GetActorLocation (Game|GetPlayerCharacter 0)) "0, 0, 0" 1.0 1.0 0.0 0 0 0 0))))

(event Collision|EventHit
  (params (MyComp :type Primitive%20Component%20Object%20Reference) (Other :type Actor%20Object%20Reference) (OtherComp :type Primitive%20Component%20Object%20Reference) (bSelfMoved :type Boolean) (HitLocation :type Vector :default "0, 0, 0") (HitNormal :type Vector :default "0, 0, 0") (NormalImpulse :type Vector :default "0, 0, 0") (Hit :type Hit%20Result%20Structure%20%28by%20ref%29))
  ;[0 0 1] Damage System.
  (Variables|Default|SetHit Hit)
  (Game|Damage|ApplyDamage (.HitActor (Collision|BreakHitResult Hit)) (Variables|Default|GetDamage) (Game|GetPlayerController 0) self "/Script/Engine.DamageType")
  (Niagara|SpawnSystematLocation (Variables|Effects|GetEmitter%20Template) HitLocation)
  (Default|CallOnProjectileImpact))

(event EventSetAttackHit
  (params (Hit :type Hit%20Result%20Structure))
  (Variables|Default|SetHit Hit))

(fn ConstructionScript
  (bind _projectilemovement (Variables|Default|GetProjectileMovement))
  (bind _speed (Variables|ProjectileSettings|GetSpeed))
  (Variables|/Script/Engine.ProjectileMovementComponent|SetInitialSpeed _projectilemovement _speed)
  (Variables|/Script/Engine.ProjectileMovementComponent|SetMaxSpeed _projectilemovement _speed)
  (Variables|/Script/Engine.ProjectileMovementComponent|SetProjectileGravityScale _projectilemovement (Variables|ProjectileSettings|GetGravity))
  (Variables|Target|GetTarget
    (:then
      (if (Variables|ProjectileSettings|GetIsHoming?)
        (Variables|/Script/Engine.ProjectileMovementComponent|SetbIsHomingProjectile _projectilemovement true)
        (Variables|/Script/Engine.ProjectileMovementComponent|SetHomingTargetComponent _projectilemovement (Variables|/Script/Engine.Actor|GetRootComponent (Variables|Target|GetTarget)))))
    (:else)))

(fn BurningDamage
  (params (HitActor :type Actor%20Object%20Reference))
  (Utilities|Time|SetTimerbyFunctionName 0 "Burning" 0.5 true)
  (CallFunction|Burning HitActor))

(fn Burning
  (params (HitActor :type Actor%20Object%20Reference))
  (Game|Damage|ApplyDamage HitActor 2.0 (Game|GetPlayerController 0) self))

(fn GetAttackHit
  (return (Variables|Default|GetHit)))