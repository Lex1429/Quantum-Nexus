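; Parent enemy character class that moves toward the player on spawn, deals melee damage and drops an XP orb on death.
; Attack sphere overlap starts a looping damage timer, gated against rapid repeats, with attack VFX, montage and sound.
; Incoming damage lowers health and triggers a one-time check of the player's weapon tags for burning or knockback.
; Death ragdolls the mesh, increments run and save kill counters, then destroys the actor.
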(event OnComponentBeginOverlap(AttackCollisionSphere)
  (params (OverlappedComponent :type Primitive%20Component%20Object%20Reference) (OtherActor :type Actor%20Object%20Reference) (OtherComp :type Primitive%20Component%20Object%20Reference) (OtherBodyIndex :type Integer) (bFromSweep :type Boolean) (SweepResult :type Hit%20Result%20Structure%20%28by%20ref%29))
  ;[1 1 1] Colliding with player starts to cause damage
  (Variables|Default|SetPlayerToDamage OtherActor)
  (bind _returnvalue (Utilities|Time|SetTimerbyFunctionName 0 "DamagePlayer" 1.0 true))
  (Variables|Default|SetDamagePlayerTimerRef _returnvalue)
  (CallFunction|DamagePlayer))

(event OnComponentEndOverlap(AttackCollisionSphere)
  (params (OverlappedComponent :type Primitive%20Component%20Object%20Reference) (OtherActor :type Actor%20Object%20Reference) (OtherComp :type Primitive%20Component%20Object%20Reference) (OtherBodyIndex :type Integer))
  ;[1 1 1] Leaving Enemy Sphere stops Damage
  (if (Utilities|Array|IsEmpty (Collision|GetOverlappingActors (Variables|Default|GetAttackCollisionSphere) "/Game/Blueprints/Characters/BP_BaseCharacterClass.BP_BaseCharacterClass_C" :!class /Script/Engine.PrimitiveComponent))
    (Utilities|Time|ClearandInvalidateTimerbyHandle (Variables|Default|GetDamagePlayerTimerRef))))

(event Custom|CountEnemies)

(event Custom|Death
  (bind _returnvalue (Game|GetPlayerCharacter 0))
  (bind _returnvalue_2 (Game|GetGameInstance))
  (bind _mesh (Variables|Character|GetMesh))
  ;[1 1 1] Death Sequence
  (Development|PrintString "Dead")
  (Game|SpawnActorfromClass "/Game/Blueprints/Items/BP_XPOrb.BP_XPOrb_C" (Math|Conversions|ToTransform(Vector) (Transformation|GetActorLocation)) "Undefined" "MultiplyWithRoot" 0 0)
  (Physics|SetSimulatePhysics _mesh true)
  (Collision|SetCollisionEnabled _mesh "QueryAndPhysics")
  (Collision|SetCollisionObjectType (Variables|Collision|GetCapsuleComponent) "ECC_GameTraceChannel6")
  (Utilities|FlowControl|Sequence
    (:then_0
      (bind _killcount (Class|BPIMissionSetup|GetRunKillCounter(Message) _returnvalue))
      (bind _result (Math|Integer|IncrementInt _killcount)
        (:%20%20
          (Class|BPIMissionSetup|SetRunKillCounter(Message) _returnvalue _result))))
    (:then_1
      (bind _killcount_2 (Class|BPIMissionSetup|GetSaveKillCounter(Message) _returnvalue_2))
      (bind _result_2 (Math|Integer|IncrementInt _killcount_2)
        (:%20%20
          (Class|BPIMissionSetup|SetSaveKillCounter(Message) _returnvalue_2 _result_2))))
    (:then_2
      (Utilities|FlowControl|Delay 0.5)
      (Actor|DestroyActor))))

(event Custom|CheckStatusEffects
  ;[0 0 1] Logic to check status effects from Damage types on weapons/abilities
  (bind _statustag (Class|BPIStatusEffects|GetWeaponStatusTag(Message) (Game|GetPlayerCharacter 0)))
  (if (GameplayTags|HasTag _statustag "(TagName=\"DamageType\")")
    (CallFunction|GetStatusEffects)))

(event Custom|DamagePlayer
  ;[1 1 1] Damage System
  (Utilities|FlowControl|DoOnce false :!label _label
    (:Completed
      (if (not (Variables|Default|GetIsDead?))
        (Game|Damage|ApplyDamage (Variables|Default|GetPlayerToDamage) (Variables|Default|GetDamage) 0 self)
        (CallFunction|EnemyAttackAnim)
        (Utilities|FlowControl|RetriggerableDelay 0.9)
        (goto _label Reset)))))

(event Custom|EnemyAttackAnim
  ;[1 1 1] Attack Animation and Sound
  (Niagara|SpawnSystematLocation (Variables|Default|GetAttackVFX) (Transformation|GetActorLocation (Variables|Default|GetPlayerToDamage)))
  (Animation|PlayAnimMontage 0 1.0 "None")
  (Audio|PlaySoundatLocation 0 "0, 0, 0" "0, 0, 0" 1.0 1.0 0.0 0 0 0 0))

(event EventBeginPlay
  ;[1 1 1] Basic Movement Towards player after spawning | TEMP
  (Utilities|FlowControl|Sequence
    (:then_0
      (AI|AIMoveTo self "0, 0, 0" (Game|GetPlayerController 0) 5.0 false))))

(event Game|Damage|EventAnyDamage
  (params (Damage :type Float%20%28single-precision%29) (DamageType :type Damage%20Type%20Object%20Reference) (InstigatedBy :type Controller%20Object%20Reference) (DamageCauser :type Actor%20Object%20Reference))
  ;[1 1 1] Damage receiver
  (Utilities|FlowControl|Sequence
    (:then_0
      (bind _output_get (Variables|Default|SetCurrentHealth (- (Variables|Default|GetCurrentHealth) Damage)))
      (if (<= _output_get 0.0)
        (Utilities|FlowControl|DoOnce false
          (:Completed
            (CallFunction|Death)))))
    (:then_1
      (Utilities|FlowControl|DoOnce false
        (:Completed
          (CallFunction|CheckStatusEffects))))))

(fn ConstructionScript)

(fn HPScale)

(fn GetStatusEffects
  (bind _statustag (Class|BPIStatusEffects|GetWeaponStatusTag(Message) (Game|GetPlayerCharacter 0)))
  (|SwitchGameplayTagContainer _statustag
    (:%28GameplayTags=%28%28TagName="DamageType.Burning"%29%29%29
      (CallFunction|BurningDamage)
      (return))
    (:%28GameplayTags=%28%28TagName="DamageType.Explosive"%29%29%29
      (CallFunction|Knockback))))

(fn BurningDamage
  (Utilities|Time|SetTimerbyFunctionName 0 "Burning" 0.5 true)
  (CallFunction|Burning))

(fn Burning
  (Game|Damage|ApplyDamage self 2.0 0 0))

(fn Knockback
  (Character|LaunchCharacter (* (Math|Vector|GetUnitDirection(Vector) (Transformation|GetActorLocation (Game|GetPlayerCharacter 0)) (Transformation|GetActorLocation)) 2.5e+03) false false))

(fn GetAbilityTag
  (return ""))

(fn GetOrbitSpawner
  (return 0))

(fn GetPlayerCurrentHealth
  (return (Variables|/Game/Blueprints/Characters/BPC_DamageSystem.BPC_DamageSystem_C|GetCurrentHealth (Variables|Default|GetBPC_DamageSystem))))

(fn GetPlayerDeathStatus
  (return (Variables|Default|GetIsDead?)))

(fn GetPlayerLevel
  (return 0))

(fn GetPlayerMaxHealth
  (return (Variables|/Game/Blueprints/Characters/BPC_DamageSystem.BPC_DamageSystem_C|GetMaxHealth (Variables|Default|GetBPC_DamageSystem))))

(fn GetPlayerXP
  (return (Variables|Default|GetCurrentXP)))

(fn GetProjectileSpawner
  (return 0))

(fn GetXptoLevel
  (return 0.0))

(fn Heal
  (params (HealAmount :type Float%20%28double-precision%29))
  (bind _newhealth (Default|Heal (Variables|Default|GetBPC_DamageSystem) HealAmount))
  (return _newhealth))

(fn TakeDamage
  (params (DamgeInfo :type BPS%20Damage%20Info%20Structure))
  (bind _wasdamaged_ (Default|TakeDamage (Variables|Default|GetBPC_DamageSystem) DamgeInfo))
  (return _wasdamaged_))