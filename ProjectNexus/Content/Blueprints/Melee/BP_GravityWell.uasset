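; BP_GravityWell is a child actor in the Melee folder that shows a portal effect and relies on parent logic for its gravity well behavior.
; On BeginPlay it attaches the teleport-portal Niagara system to its root, then calls Trigger, which only forwards to the parent.
; A separate MoveToFloor event snaps it to a Visibility trace hit, computing the trace end by multiplying its Z by -1000 rather than offsetting downward.
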(event Custom|MoveToFloor
  (bind _returnvalue (Transformation|GetActorLocation))
  (bind (_outhit _returnvalue_2) (Collision|LineTraceByChannel _returnvalue (* _returnvalue "1.000000,1.000000,-1000.000000") "TraceTypeQuery1" false (Utilities|Array|MakeArray 0) "None"))
  (if _returnvalue_2
    (Transformation|SetActorLocation (.Location (Collision|BreakHitResult _outhit)) false false)))

(event Collision|EventActorBeginOverlap
  (params (OtherActor :type Actor%20Object%20Reference)))

(event EventTick
  (params (DeltaSeconds :type Float%20%28single-precision%29)))

(event EventTrigger
  (|CallParentFunction))

(event EventBeginPlay
  (|CallParentFunction)
  (Niagara|SpawnSystemAttached "/Game/RPGEffects/ParticlesNiagara/StatusEffects/TeleportPortal/NS_Status_Teleport_Portal.NS_Status_Teleport_Portal" (Variables|Default|GetDefaultSceneRoot) "None" "0, 0, 0" "0, 0, 0" "KeepRelativeOffset" true)
  (CallFunction|Trigger))

(fn ConstructionScript
  (|CallParentFunction))